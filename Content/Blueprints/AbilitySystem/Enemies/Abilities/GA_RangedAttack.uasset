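; Enemy ranged attack gameplay ability that turns the avatar toward its combat target and fires a projectile at it.
; Through combat interface messages it captures the target's location at activation and picks a random tagged attack montage to play.
; A gameplay event matching the montage's tag, sent from an anim notify, triggers the projectile spawn at that stored location.
; The ability ends shortly after firing, or when the montage completes, is interrupted or cancelled.
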(event `self.K2_ActivateAbility`
  (bind _returnvalue (`self.GetAvatarActorFromActorInfo`))
  (bind (_taggedmontage_montage _taggedmontage_montagetag) (break `TaggedMontage` (`self.TaggedMontage`)))
  (bind _returnvalue_2 (message `EnemyInterface.GetCombatTarget` _returnvalue))
  (set `self.ProjectTileTargetLocation` (`Actor.K2_GetActorLocation` _returnvalue_2))
  (cast `CombatInterface` _returnvalue)
  (message `CombatInterface.UpdateFacingTarget` _returnvalue (`self.ProjectTileTargetLocation`))
  (bind _returnvalue_3 (message `CombatInterface.GetAttackMontages` (`self.GetAvatarActorFromActorInfo`)))
  (set `self.TaggedMontage` (`self.GetRandomTaggedMontageFromArray` _returnvalue_3))
  (`AbilityTask_PlayMontageAndWait.CreatePlayMontageAndWaitProxy` "None" _taggedmontage_montage 1.0 "None" false
    (:`then`
      ;[1 1 1] Wait for the anim notifies that hold the tag, when it gets called, the note Event Received triggered as below, check AN_MontageEvent (called in animation montage)
      (`AbilityTask_WaitGameplayEvent.WaitGameplayEvent` _taggedmontage_montagetag null
        (:`EventReceived`
          (message `CombatInterface.GetCombatSocketLocation` (`self.GetAvatarActorFromActorInfo`) _taggedmontage_montagetag)
          (`self.SpawnProjectile` (`self.ProjectTileTargetLocation`))
          (`KismetSystemLibrary.Delay` 0.5)
          (`self.K2_EndAbility`))))
    (:`OnCompleted`
      (`self.K2_EndAbility` :!label _label))
    (:`OnInterrupted`
      (goto _label))
    (:`OnCancelled`
      (goto _label))))