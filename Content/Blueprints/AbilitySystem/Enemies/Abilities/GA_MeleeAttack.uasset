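; GA_MeleeAttack is an enemy melee gameplay ability that damages hostile live players near a combat socket.
; It turns the avatar to face its combat target, plays a random tagged attack montage and waits for that montage's gameplay event.
; On the event it sphere-checks around the socket, damages non-friends and triggers their blood effect.
; Any hit fires a MeleeImpact gameplay cue; the ability ends after the check or when the montage finishes.
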(event `self.K2_ActivateAbility`
  (bind _returnvalue (`self.GetAvatarActorFromActorInfo`))
  (bind _returnvalue_2 (`self.GetAvatarActorFromActorInfo`))
  (bind (_taggedmontage_montage _taggedmontage_montagetag _taggedmontage_sockettag) (break `TaggedMontage` (`self.TaggedMontage`)))
  (bind (_taggedmontage_montage_2 _taggedmontage_montagetag_2) (break `TaggedMontage` (`self.TaggedMontage`)))
  (bind _combatsocketlocation (`self.CombatSocketLocation`))
  (set `self.HasHitTarget` false)
  (bind _returnvalue_3 (message `EnemyInterface.GetCombatTarget` _returnvalue_2))
  (set `self.CombatTarget` _returnvalue_3)
  (bind _ascombat_interface (cast `CombatInterface` _returnvalue_2))
  (`CombatInterface.UpdateFacingTarget` _ascombat_interface (`Actor.K2_GetActorLocation` _returnvalue_3))
  (bind _returnvalue_4 (message `CombatInterface.GetAttackMontages` (`self.GetAvatarActorFromActorInfo`)))
  (set `self.TaggedMontage` (`self.GetRandomTaggedMontageFromArray` _returnvalue_4))
  (`AbilityTask_PlayMontageAndWait.CreatePlayMontageAndWaitProxy` "None" _taggedmontage_montage 1.0 "None" false
    (:`then`
      (`AbilityTask_WaitGameplayEvent.WaitGameplayEvent` _taggedmontage_montagetag null
        (:`EventReceived`
          (bind _returnvalue_5 (message `CombatInterface.GetCombatSocketLocation` _returnvalue _taggedmontage_sockettag))
          (set `self.CombatSocketLocation` _returnvalue_5)
          (bind _outoverlappingactors (`AuraAbilitySystemLibrary.GetLivePlayerWithinRadius` _returnvalue (`|MakeArray` _returnvalue) 45.0 _combatsocketlocation))
          (`KismetSystemLibrary.DrawDebugSphere` _combatsocketlocation 45.0 12 (struct :`R` 1.0 :`G` 0.056774 :`A` 1.0) 2.0)
          (for _array_element _outoverlappingactors
            (if (`AuraAbilitySystemLibrary.IsNotFriend` (`self.GetAvatarActorFromActorInfo`) _array_element)
              (`self.CauseDamage` _array_element)
              (set `self.HasHitTarget` true)
              (message `CombatInterface.GetBloodEffect` _array_element)))
          (if (`self.HasHitTarget`)
            (bind _returnvalue_6 (message `EnemyInterface.GetCombatTarget` (`self.GetAvatarActorFromActorInfo`)))
            (`self.K2_ExecuteGameplayCueWithParams` (struct :`TagName` "GameplayCue.MeleeImpact") (`AbilitySystemBlueprintLibrary.MakeGameplayCueParameters` 0.0 0.0 (struct) (struct) (struct) (`BlueprintGameplayTagLibrary.MakeGameplayTagContainerFromTag` _taggedmontage_montagetag_2) (struct) (`self.CombatSocketLocation`) (0.0 0.0 0.0) null _returnvalue_6 (`self.CombatTarget`))))
          (`self.K2_EndAbility`))))
    (:`OnCompleted`
      (`self.K2_EndAbility` :!label _label))
    (:`OnInterrupted`
      (goto _label))
    (:`OnCancelled`
      (goto _label))))