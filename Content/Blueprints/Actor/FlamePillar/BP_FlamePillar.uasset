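; BP_FlamePillar is a flame pillar actor that flickers its point light to imitate a flame.
; On BeginPlay it randomly plays one of two FlameIntensity timelines, whose output scales the light's intensity relative to BaseIntensity.
; Each timeline picks again at random when it finishes, so the flicker loops continuously with a varying pattern.
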(event `self.ReceiveBeginPlay`
  (`self.ChooseTimeline`))

(event `ChooseTimeline`
  (switch `int` (`KismetMathLibrary.RandomIntegerInRange` 0 1)
    (:`Default`
      (`self.Start_2` :!label _label))
    (:`0`
      (`self.Start_1`))
    (:`1`
      (goto _label))))

(event `Start_1`
  (bind (_direction _flameintensity) (`Timeline|FlameIntensity_1` :!via `PlayFromStart`)
    (:`Update`
      (`self.Scale Flame Intensity` _flameintensity))
    (:`Finished`
      (`self.ChooseTimeline`))))

(event `Start_2`
  (bind (_direction _flameintensity) (`Timeline|FlameIntensity_2` :!via `PlayFromStart`)
    (:`Update`
      (`self.Scale Flame Intensity` _flameintensity))
    (:`Finished`
      (`self.ChooseTimeline`))))

(fn `Scale Flame Intensity`
  (params (Intensity :type "Float (double-precision)"))
  (`LightComponent.SetIntensity` (`self.PointLight`) (* Intensity (`self.BaseIntensity`))))

(fn `UserConstructionScript`)