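; Actor that fades its mesh by temporarily swapping in dynamic fade materials, running FadeOut on BeginPlay and FadeIn a second later.
; The construction script caches the original materials and creates dynamic instances from FadeMaterialInstances.
; FadeOut applies these by slot index and plays a timeline driving their "Fade" parameter, which FadeIn reverses.
; When the timeline finishes with Fade at one or above, the original materials are restored.
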(event `/Game/Blueprints/Actor/FadeActor/BI_FadeInterface.FadeOut`
  (`self.SetMaterialsToDynamicInstances`)
  (bind (_direction _fade) (`Timeline|Fade Time` :!via `PlayFromStart` :!label _label)
    (:`Update`
      (for _array_element (`self.DynamicMaterialInstances`)
        (`MaterialInstanceDynamic.SetScalarParameterValue` _array_element "Fade" _fade)))
    (:`Finished`
      (`self.FadeFinished` _fade))))

(event `/Game/Blueprints/Actor/FadeActor/BI_FadeInterface.FadeIn`
  (goto _label :!via `Reverse`))

(event `self.ReceiveBeginPlay`
  (`self.FadeOut`)
  (`KismetSystemLibrary.Delay` 1.0)
  (`self.FadeIn`))

(fn `FadeFinished`
  (params (FadeValue :type "Float (single-precision)"))
  (if (>= FadeValue 1.0)
    (`self.ResetOrginalMaterials`)
    (elif (<= FadeValue 0.0)
      _)))

(fn `ResetOrginalMaterials`
  (for (_array_element _array_index) (`self.OrginalMaterials`)
    (`PrimitiveComponent.SetMaterial` (`self.Mesh`) _array_index _array_element)))

(fn `SetMaterialsToDynamicInstances`
  (for (_array_element _array_index) (`self.DynamicMaterialInstances`)
    (`PrimitiveComponent.SetMaterial` (`self.Mesh`) _array_index _array_element)))

(fn `UserConstructionScript`
  (`KismetArrayLibrary.Array_Clear` (`self.DynamicMaterialInstances`))
  (set `self.OrginalMaterials` (`MeshComponent.GetMaterials` (`self.Mesh`)))
  (for _array_element (`self.FadeMaterialInstances`)
    (bind _returnvalue (`KismetMaterialLibrary.CreateDynamicMaterialInstance` _array_element))
    (`KismetArrayLibrary.Array_AddUnique` (`self.DynamicMaterialInstances`) _returnvalue)))